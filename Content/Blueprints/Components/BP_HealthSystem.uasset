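; BP_HealthSystem is an actor component that tracks its owner's health and plays damage feedback.
; On BeginPlay it fills health and binds to the owner's any-damage event; each hit clamps health, plays sound and particles, and fires took-damage and killed dispatchers.
; A separate Kill function spawns death burst effects.
; Heal ignores its amount and calls Heal on the owner's health component with a fixed value, never changing health.
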(event `self.ReceiveBeginPlay`
  (set `self.Owner` (`self.GetOwner`))
  (set `self.Health` (`self.MaxHealth`))
  (add `Actor.OnTakeAnyDamage` (`self.Owner`) (`|CreateDelegate` :!event `TookDamage`)))

(event `TookDamage`
  (params (DamagedActor :type "Actor Object Reference") (Damage :type "Float (single-precision)") (DamageType :type "DamageType Object Reference") (InstigatedBy :type "Controller Object Reference") (DamageCauser :type "Actor Object Reference"))
  (set `self.Health` (`KismetMathLibrary.FClamp` (- (`self.Health`) Damage) 0.0 (`self.MaxHealth`)))
  (`self.PlayFX`)
  (`self.OnTookDamage` Damage)
  (if (<= (`self.Health`) 0.0)
    (`self.OnKilled`)))

(fn `Heal`
  (params (Amountt :type "Float (double-precision)" :default 25.0))
  (bind _returnvalue (`Actor.GetComponentByClass` (`self.Owner`) "BP_HealthSystem_C"))
  (`/Engine/EditorBlueprintResources/StandardMacros.IsValid` _returnvalue
    (:`Is Valid`
      (`self.Heal` _returnvalue 25.0))))

(fn `Kill`
  (if true
    (`/Engine/EditorBlueprintResources/StandardMacros.IsValid` "/Game/Particles/PS_KillBurst.PS_KillBurst"
      (:`Is Valid`
        (`GameplayStatics.SpawnSoundAtLocation` "/Game/Audio/Kill_Cue.Kill_Cue" (`Actor.K2_GetActorLocation` (`self.Owner`)) (struct) 1.0 1.0 0.0 null null)
        (`NiagaraFunctionLibrary.SpawnSystemAtLocation` "/Game/Particles/PS_KillBurst.PS_KillBurst" (`Actor.K2_GetActorLocation` (`self.Owner`)))))))

(fn `PlayFX`
  (bind _damagedsound (`self.DamagedSound`))
  (bind _damageparticles (`self.DamageParticles`))
  (`/Engine/EditorBlueprintResources/StandardMacros.IsValid` _damagedsound
    (:`Is Valid`
      (`GameplayStatics.PlaySoundAtLocation` _damagedsound (`Actor.K2_GetActorLocation` (`self.Owner`)) (struct) 1.0 1.0 0.0 null null null null))
    (:`Is Not Valid`
      _))
  (`/Engine/EditorBlueprintResources/StandardMacros.IsValid` _damageparticles
    (:`Is Valid`
      (`NiagaraFunctionLibrary.SpawnSystemAtLocation` _damageparticles (`Actor.K2_GetActorLocation` (`self.Owner`))))))