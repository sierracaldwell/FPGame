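; Teleport system component that, in this graph, manages a regenerating stamina pool; no teleport logic is present.
; Stamina starts full on BeginPlay, and a looping timer regenerates it, clamped to the maximum.
; SpendStamina pauses that timer through PauseTickStamina, with StartTickStamina intended to resume it.
; The spend amount and resume-delay check are literal zeros, so spending deducts nothing and the resume timer is never set.
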(event `self.ReceiveBeginPlay`
  (set `self.Stamina` (`self.Max Stamina`))
  (`KismetSystemLibrary.K2_SetTimer` null "TickStamina" (`self.StaminaTickFreq`) true))

(fn `PauseTickStamina`
  (params (Duration :type "Float (double-precision)"))
  (`KismetSystemLibrary.K2_PauseTimerHandle` (`self.StaminaTickTimer`))
  (if (> 0.0 0.0)
    (`KismetSystemLibrary.K2_SetTimer` null "StartTickStamina")))

(fn `SpendStamina`
  (if (<= 0.0 (`self.Stamina`))
    (set `self.Stamina` (`KismetMathLibrary.FClamp` (- (`self.Stamina`) 0.0) 0.0 (`self.Max Stamina`)))
    (`self.PauseTickStamina` (`self.StaminaSpendPauseDuration`))))

(fn `StartTickStamina`
  (`KismetSystemLibrary.K2_UnPauseTimerHandle` (`self.StaminaTickTimer`)))

(fn `StopTickStamina`
  (`KismetSystemLibrary.K2_PauseTimerHandle` (`self.StaminaTickTimer`)))

(fn `TickStamina`
  (set `self.Stamina` (`KismetMathLibrary.FClamp` (+ (`self.Stamina`) (* (`self.StaminaRegenPerSec`) (`self.StaminaTickFreq`))) 0.0 (`self.Max Stamina`))))